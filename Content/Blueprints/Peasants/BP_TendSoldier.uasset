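; Behavior tree task in which a peasant tends a soldier, using up one medical supply.
; It snaps the character to a fixed rotation, then plays a randomly chosen tending or praying montage.
; After a delay equal to the montage length, it decrements the MedicalSupplyCount blackboard value and finishes successfully.
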(event EventReceiveExecuteAI
  (params (OwnerController :type AI%20Controller%20Object%20Reference) (ControlledPawn :type Pawn%20Object%20Reference))
  (bind _medicalsupplycount (Variables|Default|GetMedicalSupplyCount))
  (bind _ascharacter (Utilities|Casting|CastToCharacter ControlledPawn))
  (Transformation|SetActorRotation ControlledPawn "0,-120.000000, 0")
  (bind _returnvalue (Animation|PlayAnimMontage _ascharacter (Utilities|Select :Index (Math|Random|RandomInteger 2) :Option%200 "/Game/Animations/Peasants/AM_Peasant_Girl_Tender_Placement.AM_Peasant_Girl_Tender_Placement" :Option%201 "/Game/Animations/Peasants/AM_Peasant_Girl_Praying.AM_Peasant_Girl_Praying") 1.0 "None"))
  (Utilities|FlowControl|Delay _returnvalue)
  (Class|BTFunctionLibrary|SetBlackboardValueasInt _medicalsupplycount (- (Class|BTFunctionLibrary|GetBlackboardValueasInt _medicalsupplycount) 1))
  (AI|BehaviorTree|FinishExecute true))