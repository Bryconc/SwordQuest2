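; Peasant NPC tending wounded soldiers, with voiced dialogue for the Tending the Wounded quest to find fish for them.
; Conversation setup opens the pitch or a progress-based follow-up from the player's quest manager.
; Index-based Select functions supply lines and decisions, which OnDialogueEnd chains, advancing quest progress at the end.
; Decision-response logic for adding the quest or ending rudely with a scoff exists, but no event triggers it.
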(event EventAfterConversationSetup
  (bind (_dialogueindex _dialogue) (CallFunction|CreateDialogueIndexed 6))
  (bind (_decisionindex _decision) (CallFunction|CreateDecisionIndexed 3))
  (bind (_dialogueindex_2 _dialogue_2) (CallFunction|CreateDialogueIndexed))
  (bind _character (Variables|Default|GetCharacter))
  (bind _questmanagerreference (Variables|/Game/Blueprints/FirstPerson/BP_FirstPersonCharacter.BP_FirstPersonCharacter_C|GetQuestManagerReference _character))
  ;[1 1 1] Initial Dialogue
  (if (Utilities|Array|ContainsItem (Variables|/Game/QuestSystem/Blueprints/Actors/BP_QuestManager.BP_QuestManager_C|GetAllQuestClasses _questmanagerreference) "/Game/QuestSystem/Blueprints/Actors/QuestActors/Q_Tending_the_Wounded.Q_Tending_the_Wounded_C")
    (switch int (Variables|/Game/QuestSystem/Blueprints/Actors/QuestActors/BP_MasterQuest.BP_MasterQuest_C|GetCurrentProgressState (Variables|/Game/QuestSystem/Blueprints/Actors/BP_QuestManager.BP_QuestManager_C|GetCurrentQuest _questmanagerreference))
      (:0
        (CallFunction|AddDecision _decisionindex _decision))
      (:1
        (CallFunction|AddCustomImportantDialogue _dialogueindex _dialogue)))
    (else
      ;;[1 1 1] Start Quest
      (CallFunction|AddCustomImportantDialogue _dialogueindex_2 _dialogue_2))))

(event EventOnInteractwith
  (params (Character :type BP%20First%20Person%20Character%20Object%20Reference))
  ;[1 1 1] On Interact With
  (|CallParentFunction Character)
  (Variables|Default|SetCharacter Character))

(event EventOnDialogueEnd
  (params (Index :type Integer))
  (bind (_dialogueindex _dialogue) (CallFunction|CreateDialogueIndexed 5))
  (bind (_dialogueindex_2 _dialogue_2) (CallFunction|CreateDialogueIndexed 2))
  (bind (_dialogueindex_3 _dialogue_3) (CallFunction|CreateDialogueIndexed 3))
  (bind (_decisionindex _decision) (CallFunction|CreateDecisionIndexed))
  (switch int Index
    (:0
      (CallFunction|AddDecision _decisionindex _decision))
    (:1
      (CallFunction|AddCustomImportantDialogue _dialogueindex_2 _dialogue_2))
    (:2
      (CallFunction|AddCustomImportantDialogue _dialogueindex_3 _dialogue_3))
    (:3
      (CallFunction|AddDecision 0 (.Decision (CallFunction|CreateDecisionIndexed 2))))
    (:4
      (CallFunction|AddCustomImportantDialogue _dialogueindex _dialogue))
    (:5
      (CallFunction|EndConversation)
      (Variables|/Game/QuestSystem/Blueprints/Actors/QuestActors/BP_MasterQuest.BP_MasterQuest_C|SetCurrentProgressState (Variables|Default|GetAssignedQuest) 1))))

(fn ConstructionScript)

(fn CreateDialogueIndexed
  (params (Index :type Integer))
  (return Index (Utilities|Select :Index Index :Option%200 (Utilities|Struct|MakeS_DialogueInformation "/Game/Audio/Dialogue/TendingTheSoliders/PG_Beginning_1.PG_Beginning_1" "Greetings my lord. I am overjoyed to see you again. Your presence greatly encourages the men. " (Variables|Default|GetNpcName) true) :Option%201 (Utilities|Struct|MakeS_DialogueInformation "/Game/Audio/Dialogue/TendingTheSoliders/PG_Beginning_4.PG_Beginning_4" "Your father's supply of medical equipment was plenty, but we simply can't feed the wounded. They'll need some kind of nutrition or else they'll succumb to hunger. " (Variables|Default|GetNpcName) true) :Option%202 (Utilities|Struct|MakeS_DialogueInformation "/Game/Audio/Dialogue/TendingTheSoliders/PG_Beginning_5.PG_Beginning_5" "One of the scouts reported a large pond not far from here, you might search there for some fish." (Variables|Default|GetNpcName) true) :Option%203 (Utilities|Struct|MakeS_DialogueInformation "/Game/Audio/Dialogue/TendingTheSoliders/PG_Beginning_6.PG_Beginning_6" "We shouldn't need much, if you can produce just six fish, we can make them go a long way." (Variables|Default|GetNpcName) true) :Option%204 (Utilities|Struct|MakeS_DialogueInformation "/Game/Audio/Dialogue/TendingTheSoliders/PG_During_2.PG_During_2" "The scouts have told me of a large pond nearby, you should look for some fish there." (Variables|Default|GetNpcName) true) :Option%205 (Utilities|Struct|MakeS_DialogueInformation "/Game/Audio/Dialogue/TendingTheSoliders/PG_During_3.PG_During_3" "I think I saw a harpoon laying around near the medical chests, maybe you could spear some fish." (Variables|Default|GetNpcName) true) :Option%206 (Utilities|Struct|MakeS_DialogueInformation "/Game/Audio/Dialogue/TendingTheSoliders/PG_Cheese.PG_Cheese" "I like cheese!" "Mary Kathryn" false))))

(fn CreateDecisionIndexed
  (params (Index :type Integer))
  (return Index (Utilities|Select :Index Index :Option%200 (Utilities|Struct|MakeS_DecisionInformation (Utilities|Struct|MakeS_DialogueInformation "/Game/Audio/Dialogue/TendingTheSoliders/PG_Beginning_2.PG_Beginning_2" "It's been a hard march, and I fear that many have been pushed to the brink of their lives. These before me are just a few of those affected. I fear many will not last the night." (Variables|Default|GetNpcName) false) (Utilities|Array|MakeArray (Utilities|Struct|MakeS_OptionInformation "You're doing a great job, when can I expect to be ready to move out?" 0 "NewEnumerator0") (Utilities|Struct|MakeS_OptionInformation "I will not hear complaining, not while my mother is held captive and the Baron yet lives." 0 "NewEnumerator0")) false) :Option%201 (Utilities|Struct|MakeS_DecisionInformation (Utilities|Struct|MakeS_DialogueInformation "/Game/Audio/Dialogue/TendingTheSoliders/PG_Beginning_3.PG_Beginning_3" "I know you're ready to storm, and my Lady's safety is paramount, but these men need your help. They have suffered greatly over the long march." (Variables|Default|GetNpcName) true) (Utilities|Array|MakeArray (Utilities|Struct|MakeS_OptionInformation "What can I do to help? These men have put there lives on the line for me and my family. I'll do what I can." 0 "NewEnumerator0") (Utilities|Struct|MakeS_OptionInformation "I just don't have time for this" 0 "NewEnumerator0")) false) :Option%202 (Utilities|Struct|MakeS_DecisionInformation (Utilities|Struct|MakeS_DialogueInformation "/Game/Audio/Dialogue/TendingTheSoliders/PG_Beginning_7.PG_Beginning_7" "I know I had some fishing equipment laying around here somewhere. If you find it, it could probably help you. " (Variables|Default|GetNpcName) false) (Utilities|Array|MakeArray (Utilities|Struct|MakeS_OptionInformation "I'll do what I can to help." "/Game/QuestSystem/Textures/QuestIcon.QuestIcon" "NewEnumerator1") (Utilities|Struct|MakeS_OptionInformation "I really should be going." 0 "NewEnumerator0")) false) :Option%203 (Utilities|Struct|MakeS_DecisionInformation (Utilities|Struct|MakeS_DialogueInformation "/Game/Audio/Dialogue/TendingTheSoliders/PG_During_1.PG_During_1" "My lord, how goes the hunt for food?" (Variables|Default|GetNpcName) false) (Utilities|Array|MakeArray (Utilities|Struct|MakeS_OptionInformation "What exactly am I meant to be doing again?" 0 "NewEnumerator0") (Utilities|Struct|MakeS_OptionInformation "I'm still working on it" 0 "NewEnumerator0")) false) :Option%204 (Utilities|Struct|MakeS_DecisionInformation (Utilities|Struct|MakeS_DialogueInformation "/Game/Audio/Dialogue/TendingTheSoliders/PG_During_6.PG_During_6" "Would you be able to cook those on the campfire over there? It would mean the world to my patients." (Variables|Default|GetNpcName) false) (Utilities|Array|MakeArray (Utilities|Struct|MakeS_OptionInformation "Of course, they've never tasted anything like what I'll prepare!" 0 "NewEnumerator0") (Utilities|Struct|MakeS_OptionInformation "I will not cook for those that serve me!" 0 "NewEnumerator0")) false))))

(fn RudeEnding
  (Audio|PlaySoundatLocation "/Game/Audio/Dialogue/TendingTheSoliders/PG_Scoff.PG_Scoff" (Transformation|GetActorLocation) "0, 0, 0" 1.0 1.0 0.0 "/Game/Audio/Attenuation/WalkingSoundAttenuation.WalkingSoundAttenuation")
  (CallFunction|EndConversation))