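; Behavior tree task for peasant AI that loots a chest for medical supplies.
; It rotates the controlled character toward the blackboard chest location with pitch zeroed, then plays a kneel montage.
; After a delay equal to the montage's returned length, it writes a small random supply count to the blackboard, replacing the previous value, and finishes successfully.
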(event EventReceiveExecuteAI
  (params (OwnerController :type AI%20Controller%20Object%20Reference) (ControlledPawn :type Pawn%20Object%20Reference))
  (bind _returnvalue (Transformation|GetActorLocation ControlledPawn))
  (bind _chestlocation (Variables|Default|GetChestLocation))
  (bind _returnvalue_2 (Class|BTFunctionLibrary|GetBlackboardValueasVector _chestlocation))
  (bind _returnvalue_3 (Math|Rotator|FindLookatRotation _returnvalue _returnvalue_2))
  (bind (_roll _pitch _yaw) (Math|Rotator|BreakRotator _returnvalue_3))
  (bind _ascharacter (Utilities|Casting|CastToCharacter ControlledPawn))
  (Transformation|SetActorRotation ControlledPawn (Math|Rotator|MakeRotator _roll 0.0 _yaw))
  (bind _returnvalue_4 (Animation|PlayAnimMontage _ascharacter "/Game/Animations/Peasants/AM_Peasant_Girl_Kneel.AM_Peasant_Girl_Kneel" 1.0 "None"))
  (Utilities|FlowControl|Delay _returnvalue_4)
  (Class|BTFunctionLibrary|SetBlackboardValueasInt (Variables|Default|GetMedicalSuppliesCount) (Math|Random|RandomIntegerinRange 1 4))
  (AI|BehaviorTree|FinishExecute true))