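; A behavior tree task that adds occasional idle flavor to patrolling peasants.
; On execute, a one-in-four roll plays the peasant girl's pocket-search montage and a random "hmm" sound at the character's location.
; The task waits for the montage's duration before finishing successfully, or succeeds immediately when the roll fails.
; Both montage options are currently the same asset, and a failed Character cast stops without finishing the task.
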(event EventReceiveExecuteAI
  (params (OwnerController :type AI%20Controller%20Object%20Reference) (ControlledPawn :type Pawn%20Object%20Reference))
  (if (< (Math|Random|RandomFloat) 0.25)
    (bind _ascharacter (Utilities|Casting|CastToCharacter ControlledPawn))
    (bind _returnvalue (Animation|PlayAnimMontage _ascharacter (Utilities|Select :Index (Math|Random|RandomIntegerinRange 0 1) :Option%200 "/Game/Animations/Peasants/AM_Peasant_Girl_Search_Pockets.AM_Peasant_Girl_Search_Pockets" :Option%201 "/Game/Animations/Peasants/AM_Peasant_Girl_Search_Pockets.AM_Peasant_Girl_Search_Pockets") 1.0 "None"))
    (Audio|PlaySoundatLocation (Utilities|Select :Index (Math|Random|RandomIntegerinRange 0 2) :Option%200 "/Game/Audio/Dialogue/TendingTheSoliders/PG_Hmm_1.PG_Hmm_1" :Option%201 "/Game/Audio/Dialogue/TendingTheSoliders/PG_Hmm_2.PG_Hmm_2" :Option%202 "/Game/Audio/Dialogue/TendingTheSoliders/PG_Hmm_3.PG_Hmm_3") (Transformation|GetActorLocation _ascharacter))
    (Utilities|FlowControl|Delay _returnvalue))
  (AI|BehaviorTree|FinishExecute true))