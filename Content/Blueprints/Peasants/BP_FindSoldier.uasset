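; Behavior tree task for peasant AI that picks a random soldier to go to from the actors tagged SoldierTending.
; It writes an actor to the SoldierTarget blackboard key and a slightly Y-offset actor position to SoldierLocation, then finishes successfully.
; Each key uses its own random roll, so the stored location can belong to a different soldier than the stored target.
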(event EventReceiveExecuteAI
  (params (OwnerController :type AI%20Controller%20Object%20Reference) (ControlledPawn :type Pawn%20Object%20Reference))
  (bind _outactors (Actor|GetAllActorswithTag "SoldierTending"))
  (Class|BTFunctionLibrary|SetBlackboardValueasObject (Variables|Default|GetSoldierTarget) (Utilities|Array|Get(acopy) _outactors (Math|Random|RandomInteger (Utilities|Array|Length _outactors))))
  (AI|BehaviorTree|SetBlackboardValueasVector (Variables|Default|GetSoldierLocation) (+ (Transformation|GetActorLocation (Utilities|Array|Get(acopy) _outactors (Math|Random|RandomInteger (Utilities|Array|Length _outactors)))) "0,20.000000,0.000000"))
  (AI|BehaviorTree|FinishExecute true))