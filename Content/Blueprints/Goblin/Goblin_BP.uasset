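; Goblin enemy character with two bone blades that delegates walking, damage dealing and damage taking to its HostileEnemy AI controller.
; On BeginPlay it hides the blades and fills the controller's resource handler with its animations, audio, health, weapons and attack stats.
; Sword overlaps with the player deal damage and play a hit sound, gated by a time-based attack cooldown.
; Events toggle each sword's collision, and only player-instigated damage is forwarded to the controller.
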(event OnComponentBeginOverlap(RightSword)
  (params (OverlappedComponent :type Primitive%20Component%20Object%20Reference) (OtherActor :type Actor%20Object%20Reference) (OtherComp :type Primitive%20Component%20Object%20Reference) (OtherBodyIndex :type Integer) (bFromSweep :type Boolean) (SweepResult :type Hit%20Result%20Structure%20%28by%20ref%29))
  (bind _returnvalue (Game|Player|GetPlayerPawn 0))
  ;[1 1 1] Damaging Player when Swords Hit Player
  (if (== OtherActor _returnvalue)
    (bind _canattack (CallFunction|AttackSpeedValid))
    (if _canattack
      (bind _returnvalue_2 (AI|GetAIController self))
      (bind _ashostile_enemy (Utilities|Casting|CastToHostileEnemy _returnvalue_2))
      (bind _asbp_first_person_character (Utilities|Casting|CastToBP_FirstPersonCharacter _returnvalue))
      (Default|DealDamage _ashostile_enemy _asbp_first_person_character)
      (Audio|PlaySoundatLocation "/Game/Audio/NPCs/Goblin_Sword_Contact_Sound.Goblin_Sword_Contact_Sound" (Transformation|GetActorLocation))
      (Variables|Default|SetLastAttackTime (Math|DateTime|Now)))))

(event OnComponentBeginOverlap(LeftSword)
  (params (OverlappedComponent :type Primitive%20Component%20Object%20Reference) (OtherActor :type Actor%20Object%20Reference) (OtherComp :type Primitive%20Component%20Object%20Reference) (OtherBodyIndex :type Integer) (bFromSweep :type Boolean) (SweepResult :type Hit%20Result%20Structure%20%28by%20ref%29))
  (bind _returnvalue (Game|Player|GetPlayerPawn 0))
  ;[1 1 1] Damaging Player when Swords Hit Player
  (if (== OtherActor _returnvalue)
    (bind _canattack (CallFunction|AttackSpeedValid))
    (if _canattack
      (bind _returnvalue_2 (AI|GetAIController self))
      (bind _ashostile_enemy (Utilities|Casting|CastToHostileEnemy _returnvalue_2))
      (bind _asbp_first_person_character (Utilities|Casting|CastToBP_FirstPersonCharacter _returnvalue))
      (Default|DealDamage _ashostile_enemy _asbp_first_person_character)
      (Audio|PlaySoundatLocation "/Game/Audio/NPCs/Goblin_Sword_Contact_Sound.Goblin_Sword_Contact_Sound" (Transformation|GetActorLocation))
      (Variables|Default|SetLastAttackTime (Math|DateTime|Now)))))

(event Custom|DisableCollisionLeftSword
  ;[1 1 1] Sword Collision Enable/Disable
  (Collision|SetCollisionEnabled (Variables|Components|GetLeftSword) "NoCollision"))

(event Custom|EnableCollisionLeftSword
  ;[1 1 1] Sword Collision Enable/Disable
  (Collision|SetCollisionEnabled (Variables|Components|GetLeftSword) "QueryAndPhysics"))

(event Custom|EnableCollisionRightSword
  ;[1 1 1] Sword Collision Enable/Disable
  (Collision|SetCollisionEnabled (Variables|Components|GetRightSword) "QueryAndPhysics"))

(event Custom|DisableCollisionRightSword
  ;[1 1 1] Sword Collision Enable/Disable
  (Collision|SetCollisionEnabled (Variables|Components|GetRightSword) "NoCollision"))

(event EventBeginPlay
  (CallFunction|UnequipSwords)
  (bind _returnvalue (AI|GetAIController self))
  (bind _ashostile_enemy (Utilities|Casting|CastToHostileEnemy _returnvalue))
  (Default|SetWalkSpeed _ashostile_enemy)
  ;[1 1 1] Loading Assets
  (bind _returnvalue_2 (AI|GetAIController self))
  (bind _ashostile_enemy_2 (Utilities|Casting|CastToHostileEnemy _returnvalue_2))
  (bind _handler (Default|GetResourceHandler _ashostile_enemy_2))
  (Variables|Default|SetResourceHandler _handler)
  (Variables|/Script/SwordQuest2.ResourceComponent|SetAttackAnimation _handler "/Game/Animations/AnimationMontages/Goblin_Attack_1.Goblin_Attack_1")
  (Variables|/Script/SwordQuest2.ResourceComponent|SetHealth _handler (Variables|Default|GetHealth))
  (Variables|/Script/SwordQuest2.ResourceComponent|SetAgroAudio _handler "/Game/Audio/NPCs/Goblin_Scream.Goblin_Scream")
  (Variables|/Script/SwordQuest2.ResourceComponent|SetHealthWidget _handler (Variables|Components|GetAIHealth))
  (Variables|/Script/SwordQuest2.ResourceComponent|SetAttackDistance _handler (Variables|Default|GetAttackDistanceValue))
  (Variables|/Script/SwordQuest2.ResourceComponent|SetWeapon1 _handler (Variables|Components|GetBoneBlade1))
  (Variables|/Script/SwordQuest2.ResourceComponent|SetMinimumAttackDamage _handler (Variables|Default|GetMinimumDamage))
  (Variables|/Script/SwordQuest2.ResourceComponent|SetWeapon2 _handler (Variables|Components|GetBoneBlade2))
  (Variables|/Script/SwordQuest2.ResourceComponent|SetMaximumAttackDamage _handler (Variables|Default|GetMaximumDamage))
  (Variables|/Script/SwordQuest2.ResourceComponent|SetDeathAnimation _handler "/Game/Animations/AnimationMontages/Goblin_Dying.Goblin_Dying"))

(event Game|Damage|EventAnyDamage
  (params (Damage :type Float%20%28single-precision%29) (DamageType :type Damage%20Type%20Object%20Reference) (InstigatedBy :type Controller%20Object%20Reference) (DamageCauser :type Actor%20Object%20Reference))
  ;[1 1 1] Receiving Damage
  (if (== InstigatedBy (Game|GetPlayerController 0))
    (bind _returnvalue (AI|GetAIController self))
    (bind _ashostile_enemy (Utilities|Casting|CastToHostileEnemy _returnvalue))
    (Default|TakeDamage _ashostile_enemy Damage)))

(fn ConstructionScript
  (Variables|Default|SetAttackDelay (Math|Timespan|FromSeconds 2.0)))

(fn UnequipSwords
  (Rendering|SetVisibility (Variables|Components|GetBoneBlade1) false true)
  (Rendering|SetVisibility (Variables|Components|GetBoneBlade2) false true))

(fn EquipSwords
  (Rendering|SetVisibility (Variables|Components|GetBoneBlade1) true true)
  (Rendering|SetVisibility (Variables|Components|GetBoneBlade2) true true))

(fn AttackSpeedValid
  (return (> (- (Math|DateTime|Now) (Variables|Default|GetLastAttackTime)) (Variables|Default|GetAttackDelay))))