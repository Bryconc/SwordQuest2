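; Knight patroller quest NPC that offers the Goblin Assault quest through voiced conversation and reacts to its progress.
; A new player gets branching decisions and chained briefing lines, ending in the quest starting or a rude grunt exit.
; Once the quest is taken, its progress state selects a reminder, victory or follow-up line, and the victory line completes a subgoal.
; Indexed helper functions supply all lines and choices, while decision and dialogue-end events drive the flow.
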(event EventOnDecisionMade
  (params (DecisionIndex :type Integer) (ChosenOptionIndex :type Integer))
  (bind _returnvalue (- ChosenOptionIndex 1))
  (bind (_dialogueindex _dialogue) (CallFunction|CreateDialogueIndexed))
  (bind (_decisionindex _decision) (CallFunction|CreateDecisionIndexed 2))
  (switch int DecisionIndex
    (:0
      ;[1 1 1] Decision 0
      (switch int _returnvalue
        (:0
          (CallFunction|AddCustomImportantDialogue _dialogueindex _dialogue))
        (:1
          (CallFunction|RudeEnding))))
    (:1
      ;[1 1 1] Decision 1
      (switch int _returnvalue
        (:0
          (CallFunction|AddDecision _decisionindex _decision))
        (:1
          (CallFunction|RudeEnding))))
    (:2
      ;[1 1 1] Decision 2 / Quest Start
      (switch int _returnvalue
        (:0
          (CallFunction|EndConversation)
          (bind _quest (Default|AddNewQuest (Variables|/Game/Blueprints/FirstPerson/BP_FirstPersonCharacter.BP_FirstPersonCharacter_C|GetQuestManagerReference (Variables|Default|GetCharacter)) "/Game/QuestSystem/Blueprints/Actors/QuestActors/Q_Goblin_Assault.Q_Goblin_Assault_C" true))
          (CallFunction|NoLongerOfferingQuest)
          (Variables|Default|SetAssignedQuest _quest))
        (:1
          (CallFunction|RudeEnding))))))

(event EventAfterConversationSetup
  (bind (_decisionindex _decision) (CallFunction|CreateDecisionIndexed))
  (bind (_dialogueindex _dialogue) (CallFunction|CreateDialogueIndexed 5))
  (bind (_dialogueindex_2 _dialogue_2) (CallFunction|CreateDialogueIndexed 6))
  (bind (_dialogueindex_3 _dialogue_3) (CallFunction|CreateDialogueIndexed 7))
  ;[1 1 1] Initialize Conversation
  (if (Utilities|Array|ContainsItem (Variables|/Game/QuestSystem/Blueprints/Actors/BP_QuestManager.BP_QuestManager_C|GetAllQuestClasses (Variables|/Game/Blueprints/FirstPerson/BP_FirstPersonCharacter.BP_FirstPersonCharacter_C|GetQuestManagerReference (Variables|Default|GetCharacter))) "/Game/QuestSystem/Blueprints/Actors/QuestActors/Q_Goblin_Assault.Q_Goblin_Assault_C")
    (switch int (Variables|/Game/QuestSystem/Blueprints/Actors/QuestActors/BP_MasterQuest.BP_MasterQuest_C|GetCurrentProgressState (Variables|Default|GetAssignedQuest))
      (:0
        (CallFunction|AddCustomImportantDialogue _dialogueindex _dialogue))
      (:1
        (CallFunction|AddCustomImportantDialogue _dialogueindex_2 _dialogue_2)
        (Variables|/Game/QuestSystem/Blueprints/Actors/QuestActors/BP_MasterQuest.BP_MasterQuest_C|SetCurrentProgressState (Variables|Default|GetAssignedQuest) 2))
      (:2
        (CallFunction|AddCustomImportantDialogue _dialogueindex_3 _dialogue_3)))
    (else
      ;;[1 1 1] Start Quest
      (CallFunction|AddDecision _decisionindex _decision))))

(event EventOnInteractwith
  (params (Character :type BP%20First%20Person%20Character%20Object%20Reference))
  ;[1 1 1] On Interact With
  (|CallParentFunction Character)
  (Variables|Default|SetCharacter Character))

(event EventOnDialogueEnd
  (params (Index :type Integer))
  (bind (_dialogueindex _dialogue) (CallFunction|CreateDialogueIndexed 1))
  (bind (_dialogueindex_2 _dialogue_2) (CallFunction|CreateDialogueIndexed 2))
  (bind (_dialogueindex_3 _dialogue_3) (CallFunction|CreateDialogueIndexed 3))
  (bind (_dialogueindex_4 _dialogue_4) (CallFunction|CreateDialogueIndexed 4))
  (bind (_decisionindex _decision) (CallFunction|CreateDecisionIndexed 1))
  (bind (_dialogueindex_5 _dialogue_5) (CallFunction|CreateDialogueIndexed 8))
  (bind _assignedquest (Variables|Default|GetAssignedQuest))
  (switch int Index
    (:0
      (CallFunction|AddCustomImportantDialogue _dialogueindex _dialogue))
    (:1
      (CallFunction|AddCustomImportantDialogue _dialogueindex_2 _dialogue_2))
    (:2
      (CallFunction|AddCustomImportantDialogue _dialogueindex_3 _dialogue_3))
    (:3
      (CallFunction|AddCustomImportantDialogue _dialogueindex_4 _dialogue_4))
    (:4
      (CallFunction|AddDecision _decisionindex _decision))
    (:5
      (CallFunction|EndConversation :!label _label))
    (:6
      (CallFunction|EndConversation)
      (Variables|/Game/QuestSystem/Blueprints/Actors/QuestActors/BP_MasterQuest.BP_MasterQuest_C|SetCurrentProgressState _assignedquest 2)
      (Default|CompleteSubGoal _assignedquest 1 false))
    (:7
      (CallFunction|AddCustomImportantDialogue _dialogueindex_5 _dialogue_5))
    (:8
      (goto _label))))

(fn ConstructionScript
  (|CallParentFunction))

(fn CreateDialogueIndexed
  (params (Index :type Integer))
  (return Index (Utilities|Select :Index Index :Option%200 (Utilities|Struct|MakeS_DialogueInformation "/Game/Audio/Dialogue/GoblinAssualt/GA_B_2.GA_B_2" "I'm afraid we have a bit of a problem there. These woods are infested with Goblins." (Variables|Default|GetNpcName)) :Option%201 (Utilities|Struct|MakeS_DialogueInformation "/Game/Audio/Dialogue/GoblinAssualt/GA_B_3.GA_B_3" "They have given us problems for years, attacking villages in the night and stealing our supplies." (Variables|Default|GetNpcName)) :Option%202 (Utilities|Struct|MakeS_DialogueInformation "/Game/Audio/Dialogue/GoblinAssualt/GA_B_4.GA_B_4" "At the moment we're the only thing standing between them and your castle." (Variables|Default|GetNpcName)) :Option%203 (Utilities|Struct|MakeS_DialogueInformation "/Game/Audio/Dialogue/GoblinAssualt/GA_B_5.GA_B_5" "If we ignore them now, we've left our home defenceless and they're sure to hurt more of your people." (Variables|Default|GetNpcName)) :Option%204 (Utilities|Struct|MakeS_DialogueInformation "/Game/Audio/Dialogue/GoblinAssualt/GA_B_6.GA_B_6" "I'm afraid most of my unit is too exhausted from the journey to handle this." (Variables|Default|GetNpcName)) :Option%205 (Utilities|Struct|MakeS_DialogueInformation "/Game/Audio/Dialogue/GoblinAssualt/GA_D_1.GA_D_1" "How goes the hunt? I can still hear they're awful snarl. We can't leave until they've been eliminated" (Variables|Default|GetNpcName)) :Option%206 (Utilities|Struct|MakeS_DialogueInformation "/Game/Audio/Dialogue/GoblinAssualt/GA_E_1.GA_E_1" "Huzzah! My lord remains victorious. Your skill in combat has surely inspired morale." (Variables|Default|GetNpcName)) :Option%207 (Utilities|Struct|MakeS_DialogueInformation "/Game/Audio/Dialogue/GoblinAssualt/GA_P_1.GA_P_1" "From the way you handled those goblins, I am proud to serve you. We continue to fight at your side." (Variables|Default|GetNpcName)) :Option%208 (Utilities|Struct|MakeS_DialogueInformation "/Game/Audio/Dialogue/GoblinAssualt/GA_P_2.GA_P_2" "Let us know when you're ready to move." (Variables|Default|GetNpcName)))))

(fn CreateDecisionIndexed
  (params (Index :type Integer))
  (return Index (Utilities|Select :Index Index :Option%200 (Utilities|Struct|MakeS_DecisionInformation (Utilities|Struct|MakeS_DialogueInformation "/Game/Audio/Dialogue/GoblinAssualt/GA_B_1.GA_B_1" "My lord. How may I serve you?" (Variables|Default|GetNpcName)) (Utilities|Array|MakeArray (Utilities|Struct|MakeS_OptionInformation "We have set camp here for the night. When will we be ready to move?" 0 "NewEnumerator0") (Utilities|Struct|MakeS_OptionInformation "On your way. I have nothing to say to you." 0 "NewEnumerator0")) false) :Option%201 (Utilities|Struct|MakeS_DecisionInformation (Utilities|Struct|MakeS_DialogueInformation "/Game/Audio/Dialogue/GoblinAssualt/GA_B_7.GA_B_7" "We won't be ready to move until these menace are dealt with." (Variables|Default|GetNpcName)) (Utilities|Array|MakeArray (Utilities|Struct|MakeS_OptionInformation "How can I help?" 0 "NewEnumerator0") (Utilities|Struct|MakeS_OptionInformation "One of you deal with it. I'm far too busy." 0 "NewEnumerator0")) false) :Option%202 (Utilities|Struct|MakeS_DecisionInformation (Utilities|Struct|MakeS_DialogueInformation "/Game/Audio/Dialogue/GoblinAssualt/GA_B_8.GA_B_8" "This would be a fine opportunity to show off your skill in combat. Slay all the beast that dwell in the woods." (Variables|Default|GetNpcName)) (Utilities|Array|MakeArray (Utilities|Struct|MakeS_OptionInformation "You don't need to ask a second time." "/Game/QuestSystem/Textures/QuestIcon.QuestIcon" "NewEnumerator1") (Utilities|Struct|MakeS_OptionInformation "I won't waste my time." 0 "NewEnumerator0")) false))))

(fn RudeEnding
  (Audio|PlaySoundatLocation "/Game/Audio/Dialogue/GoblinAssualt/GA_Grunt.GA_Grunt" (Transformation|GetActorLocation) "0, 0, 0" 1.0 1.0 0.0 "/Game/Audio/Attenuation/WalkingSoundAttenuation.WalkingSoundAttenuation")
  (CallFunction|EndConversation))