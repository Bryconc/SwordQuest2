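; BP_Harpoon is a melee-style harpoon weapon with its own hit response for swimming fish.
; Its construction script sets the attack delay, base damage and arm strike animation.
; HitTarget intercepts BP_SwimmingFish hits, checks attack speed, records the attack time and only prints a placeholder debug string, applying no damage there.
; All other targets go to the parent class's HitTarget.
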(event EventHitTarget
  (params (DamagedActor :type Actor%20Object%20Reference))
  (Utilities|Casting|CastToBP_SwimmingFish DamagedActor
    (:then
      (if (CallFunction|AttackSpeedValid)
        (Variables|Default|SetLastAttackTime (Math|DateTime|Now))
        (Development|PrintString "Hello")))
    (:CastFailed
      (|CallParentFunction DamagedActor))))

(fn ConstructionScript
  (Variables|Default|SetAttackDelay (Math|Timespan|FromSeconds 1.0))
  (Variables|Default|SetBaseDamage 0.05)
  (Variables|Default|SetAttackAnimation (Utilities|Array|MakeArray "/Game/Animations/AnimationMontages/AM_Arms_Harpoon_Strike.AM_Arms_Harpoon_Strike")))