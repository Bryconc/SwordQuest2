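; BP_MasterWeapon is a melee weapon, apparently meant as a base class, that damages actors its capsule overlaps.
; EnableSword and DisableSword toggle the capsule's collision to open and close the hit window.
; Overlaps feed HitTarget, which skips player 0's character and allows one hit per AttackDelay across all targets.
; Damage is always instigated by player controller 0, with the parent actor as causer.
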(event OnComponentBeginOverlap(Capsule)
  (params (OverlappedComponent :type Primitive%20Component%20Object%20Reference) (OtherActor :type Actor%20Object%20Reference) (OtherComp :type Primitive%20Component%20Object%20Reference) (OtherBodyIndex :type Integer) (bFromSweep :type Boolean) (SweepResult :type Hit%20Result%20Structure%20%28by%20ref%29))
  (CallFunction|HitTarget OtherActor))

(event Custom|DisableSword
  (Collision|SetCollisionEnabled (Variables|Default|GetCapsule) "NoCollision"))

(event Custom|EnableSword
  (Collision|SetCollisionEnabled (Variables|Default|GetCapsule) "QueryAndPhysics"))

(fn ConstructionScript)

(fn AttackSpeedValid
  (return (> (- (Math|DateTime|Now) (Variables|Default|GetLastAttackTime)) (Variables|Default|GetAttackDelay))))

(fn HitTarget
  (params (DamagedActor :type Actor%20Object%20Reference))
  (if (!= DamagedActor (Game|GetPlayerCharacter 0))
    (if (CallFunction|AttackSpeedValid)
      (Variables|Default|SetLastAttackTime (Math|DateTime|Now))
      (Game|Damage|ApplyDamage DamagedActor (Variables|Default|GetBaseDamage) (Game|GetPlayerController 0) (Actor|GetParentActor)))))