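; Behavior tree task that puts a hostile enemy into combat and charges it at its target.
; On first execution it casts and caches the owner as HostileEnemy, then equips weapons, sets the InCombat blackboard flag, adjusts walk speed and plays aggro audio.
; AIMoveTo chases the TargetToFollow actor to within the resource handler's attack distance.
; Success finishes the task; failure clears the target and fails it.
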(event EventReceiveExecute
  (params (OwnerActor :type Actor%20Object%20Reference))
  (if (!= (Variables|Default|GetAI_CON_Ref) 0)
    _
    (else
      (bind _ashostile_enemy (Utilities|Casting|CastToHostileEnemy OwnerActor))
      (Variables|Default|SetAI_CON_Ref _ashostile_enemy)))
  (bind _handler (Default|GetResourceHandler _ashostile_enemy))
  ;[1 1 1] Battle Ready
  (Default|EquipWeapons _ashostile_enemy)
  (Class|BTFunctionLibrary|SetBlackboardValueasBool (Variables|Default|GetInCombat) true)
  (Default|SetWalkSpeed (Variables|Default|GetAI_CON_Ref))
  (Audio|PlaySoundatLocation (Variables|/Script/SwordQuest2.ResourceComponent|GetAgroAudio _handler) (Transformation|GetActorLocation (Pawn|GetControlledPawn (Variables|Default|GetAI_CON_Ref))))
  (AI|AIMoveTo (Pawn|GetControlledPawn (Variables|Default|GetAI_CON_Ref)) "0, 0, 0" (AI|BehaviorTree|GetBlackboardValueasActor (Variables|Default|GetTargetToFollow)) (Variables|/Script/SwordQuest2.ResourceComponent|GetAttackDistance _handler) false
    (:OnSuccess
      (AI|BehaviorTree|FinishExecute true))
    (:OnFail
      (Class|BTFunctionLibrary|SetBlackboardValueasObject (Variables|Default|GetTargetToFollow))
      (AI|BehaviorTree|FinishExecute false))))