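; AI controller for a hostile enemy that runs the follower behavior tree and stores its home location in the blackboard on possession-independent BeginPlay.
; A Resource object supplies health, random damage range, weapons, death montage and health widget.
; Tick handles one-time death or updates the health bar, shown in combat and turned toward the player.
; The InCombat key also sets walk speed; functions toggle weapon visibility.
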(event Custom|TakeDamage
  (params (DamageTaken :type Float%20%28single-precision%29))
  (bind _resource (Variables|Default|GetResource))
  ;[1 1 1] Receive Damage
  (Variables|/Script/SwordQuest2.ResourceComponent|SetHealth _resource (- (Variables|/Script/SwordQuest2.ResourceComponent|GetHealth _resource) DamageTaken)))

(event Custom|DealDamage
  (params (PlayerToDamage :type BP%20First%20Person%20Character%20Object%20Reference))
  (bind _resource (Variables|Default|GetResource))
  ;[1 1 1] Deal Damage to Target
  (Game|Damage|ApplyDamage PlayerToDamage (Math|Random|RandomFloatinRange (Variables|/Script/SwordQuest2.ResourceComponent|GetMinimumAttackDamage _resource) (Variables|/Script/SwordQuest2.ResourceComponent|GetMaximumAttackDamage _resource)) self 0 "/Script/Engine.DamageType"))

(event Custom|SetWalkSpeed
  ;[1 1 1] Set Walk Speed by Combat
  (bind _ascharacter (Utilities|Casting|CastToCharacter (Pawn|GetControlledPawn self)))
  (if (ScalableFloat|GetValueasBool (Variables|Default|GetBlackboard) (Variables|Default|GetinCombat))
    (Variables|/Script/Engine.CharacterMovementComponent|SetMaxWalkSpeed (Variables|/Script/Engine.Character|GetCharacterMovement _ascharacter) 8e+02)
    (else
      (Variables|/Script/Engine.CharacterMovementComponent|SetMaxWalkSpeed (Variables|/Script/Engine.Character|GetCharacterMovement _ascharacter) 2e+02))))

(event EventTick
  (params (DeltaSeconds :type Float%20%28single-precision%29))
  (bind _returnvalue (Game|GetPlayerCharacter 0))
  (bind _self self)
  (bind _resource (Variables|Default|GetResource))
  (bind _resource_2 (Variables|Default|GetResource))
  (bind _resource_3 (Variables|Default|GetResource))
  (bind _returnvalue_2 (Transformation|GetActorLocation _returnvalue))
  (bind _healthwidget (Variables|/Script/SwordQuest2.ResourceComponent|GetHealthWidget _resource))
  (bind _deathanimation (Variables|/Script/SwordQuest2.ResourceComponent|GetDeathAnimation _resource_2))
  (bind _returnvalue_3 (Transformation|GetWorldLocation _healthwidget))
  (bind _returnvalue_4 (Math|Rotator|FindLookatRotation _returnvalue_3 _returnvalue_2))
  (bind (_roll _pitch _yaw) (Math|Rotator|BreakRotator _returnvalue_4))
  (if (and (<= (Variables|/Script/SwordQuest2.ResourceComponent|GetHealth (Variables|Default|GetResource)) 0.0) (Variables|Default|GetAlive))
    ;[1 1 1] Process Death
    (Variables|Default|SetAlive false)
    (bind _ascharacter (Utilities|Casting|CastToCharacter (Pawn|GetControlledPawn _self)))
    (CallFunction|UnequipWeapons _self)
    (Animation|PlayAnimMontage _ascharacter _deathanimation 1.0 "None")
    (Development|PrintString (Utilities|GetDisplayName _deathanimation))
    (else
      ;[1 1 1] Update Health Bar
      (bind _asaihealth (Utilities|Casting|CastToAIHealth (UserInterface|GetUserWidgetObject (Variables|/Script/SwordQuest2.ResourceComponent|GetHealthWidget _resource_3))))
      (if (ScalableFloat|GetValueasBool (stale EventBeginPlay _blackboardcomponent) (Variables|Default|GetinCombat))
        (Default|ShowHealthBar _asaihealth)
        (else
          (Default|RemoveHealthBar _asaihealth)))
      (Progress|SetPercent (Variables|/Game/Widgets/AIHealth.AIHealth_C|GetAIHealthBar _asaihealth) (Variables|/Script/SwordQuest2.ResourceComponent|GetHealth _resource_3))
      ;[1 1 1] Keep Health Bar Facing Player
      (Transformation|SetWorldRotation _healthwidget (Math|Rotator|MakeRotator _roll 0.0 _yaw) false false))))

(event EventBeginPlay
  ;[1 1 1] Setup Blackboard
  (bind _blackboardcomponent (Class|AIController|UseBlackboard "/Game/Blueprints/ArtificialIntelligence/FollowerBlackboard.FollowerBlackboard"))
  (AI|Components|Blackboard|SetValueasVector _blackboardcomponent (Variables|Default|GetHomeLocation) (Transformation|GetActorLocation (Pawn|GetControlledPawn)))
  (AI|RunBehaviorTree "/Game/Blueprints/ArtificialIntelligence/FollowerBT.FollowerBT"))

(fn ConstructionScript
  (Variables|Default|SetAlive true))

(fn GetResourceHandler
  (return (Variables|Default|GetResource)))

(fn EquipWeapons
  (bind _resource (Variables|Default|GetResource))
  (bind _weapon1 (Variables|/Script/SwordQuest2.ResourceComponent|GetWeapon1 _resource))
  (bind _weapon2 (Variables|/Script/SwordQuest2.ResourceComponent|GetWeapon2 _resource))
  (Utilities|IsValid _weapon1
    (:Is%20Valid
      (Rendering|SetVisibility _weapon1 true true)
      (Utilities|IsValid _weapon2
        (:Is%20Valid
          (Rendering|SetVisibility _weapon2 true true))))))

(fn UnequipWeapons
  (bind _resource (Variables|Default|GetResource))
  (bind _weapon1 (Variables|/Script/SwordQuest2.ResourceComponent|GetWeapon1 _resource))
  (bind _weapon2 (Variables|/Script/SwordQuest2.ResourceComponent|GetWeapon2 _resource))
  (Utilities|IsValid _weapon1
    (:Is%20Valid
      (Rendering|SetVisibility _weapon1 false true)
      (Utilities|IsValid _weapon2
        (:Is%20Valid
          (Rendering|SetVisibility _weapon2 false true))))))