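; Goblin NPC character driven by the Follower_AI_CON AI controller.
; On BeginPlay it hides both bone blade components, hands the goblin scream to the controller as its aggro audio, and applies the base walk speed.
; Every Tick it sets movement speed from the IsSprinting flag, switching between a hardcoded sprint speed and BaseWalkSpeed.
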(event EventTick
  (params (DeltaSeconds :type Float%20%28single-precision%29))
  (bind _charactermovement (Variables|Character|GetCharacterMovement))
  (if (Variables|Default|GetisSprinting)
    (Variables|/Script/Engine.CharacterMovementComponent|SetMaxWalkSpeed _charactermovement 6e+02)
    (else
      (Variables|/Script/Engine.CharacterMovementComponent|SetMaxWalkSpeed _charactermovement (Variables|Default|GetBaseWalkSpeed)))))

(event EventBeginPlay
  (bind _self self)
  (Rendering|SetVisibility (Variables|Default|GetBoneBlade1 _self) false true)
  (Rendering|SetVisibility (Variables|Default|GetBoneBlade2 _self) false true)
  (bind _returnvalue (AI|GetAIController _self))
  (bind _asfollower_ai_con (Utilities|Casting|CastToFollower_AI_CON _returnvalue))
  (Variables|/Game/Blueprints/ArtificialIntelligence/Follower_AI_CON.Follower_AI_CON_C|SetAgroAudio _asfollower_ai_con "/Game/Audio/NPCs/Goblin_Scream.Goblin_Scream")
  ;[1 1 1] Set NPC Base Walk Speed
  (bind _ascharacter (Utilities|Casting|CastToCharacter (Pawn|GetControlledPawn _returnvalue)))
  (Variables|/Script/Engine.CharacterMovementComponent|SetMaxWalkSpeed (Variables|/Script/Engine.Character|GetCharacterMovement _ascharacter) (Variables|Default|GetBaseWalkSpeed)))

(fn ConstructionScript)