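; Behavior tree decorator for hostile enemy AI that tests the distance between the controlled pawn and its TargetToFollow against the resource handler's AttackDistance.
; Despite its name, it passes while the target is at or beyond that distance.
; As a side effect, each check sets the InCombat blackboard key to the inverse result and calls SetWalkSpeed through AICONRef.
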(fn PerformConditionCheckAI
  (params (OwnerController :type AI%20Controller%20Object%20Reference) (ControlledPawn :type Pawn%20Object%20Reference))
  (bind _ashostile_enemy (Utilities|Casting|CastToHostileEnemy OwnerController))
  (bind _handler (Default|GetResourceHandler _ashostile_enemy))
  (Class|BTFunctionLibrary|SetBlackboardValueasBool (Variables|Default|GetInCombat) (not (>= (Math|Vector|VectorLength (- (Transformation|GetActorLocation (AI|BehaviorTree|GetBlackboardValueasActor (Variables|Default|GetTargetToFollow))) (Transformation|GetActorLocation ControlledPawn))) (Variables|/Script/SwordQuest2.ResourceComponent|GetAttackDistance _handler))))
  (Default|SetWalkSpeed (Variables|Default|GetAI_CON_Ref))
  (return (>= (Math|Vector|VectorLength (- (Transformation|GetActorLocation (AI|BehaviorTree|GetBlackboardValueasActor (Variables|Default|GetTargetToFollow))) (Transformation|GetActorLocation ControlledPawn))) (Variables|/Script/SwordQuest2.ResourceComponent|GetAttackDistance _handler))))