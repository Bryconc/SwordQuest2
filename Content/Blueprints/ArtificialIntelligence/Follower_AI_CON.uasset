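; AI controller for follower pawns, driving them through the FollowerBT behavior tree.
; On BeginPlay it initializes FollowerBlackboard, stores the controlled pawn's current location as HomeLocation, then runs the tree.
; A GetResourceHandler function exposes the controller's Resource variable.
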(event EventBeginPlay
  (Class|AIController|UseBlackboard "/Game/Blueprints/ArtificialIntelligence/FollowerBlackboard.FollowerBlackboard")
  (AI|Components|Blackboard|SetValueasVector (AI|GetBlackboard self) (Variables|Default|GetHomeLocation) (Transformation|GetActorLocation (Pawn|GetControlledPawn)))
  (AI|RunBehaviorTree "/Game/Blueprints/ArtificialIntelligence/FollowerBT.FollowerBT"))

(fn ConstructionScript)

(fn GetResourceHandler
  (return (Variables|Default|GetResource)))