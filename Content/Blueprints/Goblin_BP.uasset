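; Goblin enemy character driven by Follower_AI_CON, with two swords that detect hits on the player.
; On BeginPlay it hides both bone blades and loads its attack animation, aggro scream and attack range into the AI controller's resource handler.
; Tick switches walk speed by sprint state.
; Exposed events toggle each sword's collision, and either sword overlapping the player calls Test on BP_FirstPersonCharacter.
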(event OnComponentBeginOverlap(RightSword)
  (params (OverlappedComponent :type Primitive%20Component%20Object%20Reference) (OtherActor :type Actor%20Object%20Reference) (OtherComp :type Primitive%20Component%20Object%20Reference) (OtherBodyIndex :type Integer) (bFromSweep :type Boolean) (SweepResult :type Hit%20Result%20Structure%20%28by%20ref%29))
  (bind _returnvalue (Game|Player|GetPlayerPawn 0))
  (if (== OtherActor _returnvalue)
    (bind _asbp_first_person_character (Utilities|Casting|CastToBP_FirstPersonCharacter _returnvalue))
    (Default|Test _asbp_first_person_character)))

(event OnComponentBeginOverlap(LeftSword)
  (params (OverlappedComponent :type Primitive%20Component%20Object%20Reference) (OtherActor :type Actor%20Object%20Reference) (OtherComp :type Primitive%20Component%20Object%20Reference) (OtherBodyIndex :type Integer) (bFromSweep :type Boolean) (SweepResult :type Hit%20Result%20Structure%20%28by%20ref%29))
  (bind _returnvalue (Game|Player|GetPlayerPawn 0))
  (if (== OtherActor _returnvalue)
    (bind _asbp_first_person_character (Utilities|Casting|CastToBP_FirstPersonCharacter _returnvalue))
    (Default|Test _asbp_first_person_character)))

(event Custom|DisableCollisionLeftSword
  ;[1 1 1] Sword Collision Enable/Disable
  (Collision|SetCollisionEnabled (Variables|Default|GetLeftSword) "NoCollision"))

(event Custom|EnableCollisionLeftSword
  ;[1 1 1] Sword Collision Enable/Disable
  (Collision|SetCollisionEnabled (Variables|Default|GetLeftSword) "QueryAndPhysics"))

(event Custom|EnableCollisionRightSword
  ;[1 1 1] Sword Collision Enable/Disable
  (Collision|SetCollisionEnabled (Variables|Default|GetRightSword) "QueryAndPhysics"))

(event Custom|DisableCollisionRightSword
  ;[1 1 1] Sword Collision Enable/Disable
  (Collision|SetCollisionEnabled (Variables|Default|GetRightSword) "NoCollision"))

(event EventTick
  (params (DeltaSeconds :type Float%20%28single-precision%29))
  (bind _charactermovement (Variables|Character|GetCharacterMovement))
  ;[1 1 1] Change Walk Speed Based on Sprinting
  (if (Variables|Default|GetisSprinting)
    (Variables|/Script/Engine.CharacterMovementComponent|SetMaxWalkSpeed _charactermovement 6e+02)
    (else
      (Variables|/Script/Engine.CharacterMovementComponent|SetMaxWalkSpeed _charactermovement (Variables|Default|GetBaseWalkSpeed)))))

(event EventBeginPlay
  (bind _self self)
  (Variables|Default|SetAlive true)
  ;[1 1 1] Swords Initially Invisible
  (Rendering|SetVisibility (Variables|Default|GetBoneBlade1 _self) false true)
  (Rendering|SetVisibility (Variables|Default|GetBoneBlade2 _self) false true)
  ;[1 1 1] Loading Assets
  (bind _returnvalue (AI|GetAIController _self))
  (bind _asfollower_ai_con (Utilities|Casting|CastToFollower_AI_CON _returnvalue))
  (bind _handler (Default|GetResourceHandler _asfollower_ai_con))
  (Variables|/Script/SwordQuest2.ResourceComponent|SetAttackAnimation _handler "/Game/Animations/AnimationMontages/Goblin_Attack_1.Goblin_Attack_1")
  (Variables|/Script/SwordQuest2.ResourceComponent|SetAgroAudio _handler "/Game/Audio/NPCs/Goblin_Scream.Goblin_Scream")
  (Variables|/Script/SwordQuest2.ResourceComponent|SetAttackDistance _handler 2e+02))

(fn ConstructionScript)