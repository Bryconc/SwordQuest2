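; BP_MasterNPC is an NPC Blueprint that shows an overhead name and hands a quest to the interacting character.
; BeginPlay sets the question mark's visibility from HasQuestIcon and writes Name into the InteractionWidget.
; Player-radius events show and hide that widget.
; Interaction adds and starts the hardcoded Quest_Test1 through the character's quest manager if not already present, then hides the question mark.
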(event EventOnEnterPlayerRadius
  (params (Character :type BP%20First%20Person%20Character%20Object%20Reference))
  ;[1 1 1] Add/Remove Overhead
  (Rendering|SetVisibility (Variables|Default|GetInteractionWidget) true false))

(event EventOnLeavePlayerRadius
  (params (Character :type BP%20First%20Person%20Character%20Object%20Reference))
  ;[1 1 1] Add/Remove Overhead
  (Rendering|SetVisibility (Variables|Default|GetInteractionWidget) false false))

(event EventBeginPlay
  ;[1 1 1] Show Quest Icon
  (Rendering|SetVisibility (Variables|Default|GetQuestionMark) (Variables|Default|GetHasQuestIcon) false)
  ;[1 1 1] Set Name on Overhead Widget
  (bind _asinteraction_widget (Utilities|Casting|CastToInteractionWidget (UserInterface|GetUserWidgetObject (Variables|Default|GetInteractionWidget))))
  (Rendering|Components|TextRender|SetText (Variables|/Game/QuestSystem/Widgets/InteractionWidget.InteractionWidget_C|GetName _asinteraction_widget) (Variables|Default|GetName)))

(event EventOnInteractwith
  (params (Character :type BP%20First%20Person%20Character%20Object%20Reference))
  (bind _questmanagerreference (Variables|/Game/Blueprints/FirstPerson/BP_FirstPersonCharacter.BP_FirstPersonCharacter_C|GetQuestManagerReference Character))
  ;[1 1 1] Assign Quest
  (if (not (Utilities|Array|ContainsItem (Variables|/Game/QuestSystem/Blueprints/Actors/BP_QuestManager.BP_QuestManager_C|GetAllQuestClasses _questmanagerreference) "/Game/QuestSystem/Blueprints/Actors/QuestActors/Quest_Test1.Quest_Test1_C"))
    (Default|AddNewQuest _questmanagerreference "/Game/QuestSystem/Blueprints/Actors/QuestActors/Quest_Test1.Quest_Test1_C" true)
    (Rendering|SetVisibility (Variables|Default|GetQuestionMark) false false)))

(fn ConstructionScript)