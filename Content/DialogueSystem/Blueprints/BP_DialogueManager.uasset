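; Dialogue manager that plays voiced lines and player decisions through the HUD's dialogue and decision widgets.
; AddSimpleDialogue and AddDecision play 2D audio, with parallel delays for optional skipping and end-of-line handling.
; State flags gate continue and number-key input; finished lines and chosen options are reported back to Character.
; OnDecisionSpoken is an empty stub, and the timers OnDecisionMade clears are never started here.
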(event Custom|HandleContinueCommand
  ;[1 1 1] Handle Continue Command
  (if (Variables|Default|GetWaitingForInput)
    (if (Variables|Default|GetIsCurrentDecision)
      (if (Variables|Default|GetDialogueFinished)
        (CallFunction|OnContinueDialogue)
        (else
          (CallFunction|OnDialogueSpoken)))
      (elif (Variables|Default|GetDecisionFinished)
        (CallFunction|OnDecisionMade (Variables|/Game/DialogueSystem/Widgets/DecisionDialogue.DecisionDialogue_C|GetCurrentSelectedIndex (Variables|Default|GetDecisionWidget)))
        (else
          (CallFunction|OnDecisionSpoken))))))

(event Custom|OnDialogueSpoken
  (bind _dialoguewidget (Variables|Default|GetDialogueWidget))
  (bind _currentsound (Variables|Default|GetCurrentSound))
  ;[1 1 1] On Dialogue Spoken
  (if (and (not (Variables|Default|GetDialogueFinished)) (Variables|Default|GetIsCurrentDialogue))
    (Variables|Default|SetDialogueFinished true)
    (Variables|Default|SetWaitingForInput true)
    (Widget|SetVisibility (Variables|/Game/DialogueSystem/Widgets/DefaultDialogue.DefaultDialogue_C|GetSpaceText _dialoguewidget) "Hidden")
    (Widget|SetVisibility (Variables|/Game/DialogueSystem/Widgets/DefaultDialogue.DefaultDialogue_C|GetContinueArrow _dialoguewidget) "Visible")
    (Utilities|IsValid _currentsound
      (:Is%20Valid
        (Audio|Components|Audio|Stop _currentsound)
        (Components|DestroyComponent _currentsound)))))

(event Custom|HandleNumberKey
  (params (NumberPressed :type Integer))
  (bind _returnvalue (- NumberPressed 1))
  ;[1 1 1] Handle Number Keys (0-9)
  (if (Math|Boolean|ANDBoolean (Variables|Default|GetWaitingForInput) (Variables|Default|GetDecisionFinished) (Variables|Default|GetIsCurrentDecision))
    (if (and (> NumberPressed 0) (<= NumberPressed (Utilities|Array|Length (Variables|/Game/DialogueSystem/Widgets/DecisionDialogue.DecisionDialogue_C|GetOptionsWidgets (Variables|Default|GetDecisionWidget)))))
      (Variables|Default|SetWaitingForInput false)
      (Default|SelectOption (Variables|Default|GetDecisionWidget) _returnvalue)
      (CallFunction|OnDecisionMade _returnvalue))))

(event Custom|AddSimpleDialogue
  (params (Dialogue :type S%20Dialogue%20Information%20Structure) (Index :type Integer))
  (bind (_audiofile _spokentext _sendername _canbeskipped _skiptime) (Utilities|Struct|BreakS_DialogueInformation Dialogue))
  ;[1 1 1] Add Simple Dialogue
  (if (not (Variables|Default|GetIsCurrentDialogue))
    (Variables|Default|SetIsCurrentDialogue true)
    (Variables|Default|SetCurrentDialogueIndex Index)
    (Utilities|IsValid _audiofile
      (:Is%20Valid
        (bind _returnvalue (Audio|SpawnSound2D _audiofile))
        (Variables|Default|SetCurrentSound _returnvalue)
        (Default|ShowNewMessage (Variables|Default|GetDialogueWidget) _sendername _spokentext)
        (Utilities|FlowControl|Sequence
          (:then_0
            (if _canbeskipped
              (Utilities|FlowControl|Delay _skiptime)
              (Variables|Default|SetWaitingForInput true)
              (Widget|SetVisibility (Variables|/Game/DialogueSystem/Widgets/DefaultDialogue.DefaultDialogue_C|GetSpaceText (Variables|Default|GetDialogueWidget)) "Visible")))
          (:then_1
            (Utilities|FlowControl|Delay (select (Utilities|IsValid _audiofile) (Variables|/Script/Engine.SoundBase|GetDuration _audiofile) 2.0))
            (CallFunction|OnDialogueSpoken)))))))

(event Custom|OnDecisionMade
  (params (OptionIndex :type Integer))
  (bind _returnvalue (Game|GetPlayerController 0))
  (bind _decisionwidget (Variables|Default|GetDecisionWidget))
  (bind _decisionwidget_2 (Variables|Default|GetDecisionWidget))
  (bind _blendin (Variables|/Game/DialogueSystem/Widgets/DecisionDialogue.DecisionDialogue_C|GetBlendIn _decisionwidget_2))
  ;[1 1 1] On Decision Made
  (Utilities|FlowControl|DoOnce false :!label _label
    (:Completed
      (Utilities|Time|ClearandInvalidateTimerbyHandle (Variables|Default|GetIntTimer))
      (Variables|Default|SetWaitingForInput false)
      (Utilities|Time|ClearandInvalidateTimerbyHandle (Variables|Default|GetFloatTimer))
      (Variables|Default|SetChosenOption OptionIndex)
      (Widget|SetVisibility (Variables|/Game/DialogueSystem/Widgets/DecisionDialogue.DecisionDialogue_C|GetOptionsBox (Variables|Default|GetDecisionWidget)) "Hidden")
      (Variables|/Script/Engine.PlayerController|SetbEnableClickEvents _returnvalue false)
      (Variables|/Script/Engine.PlayerController|SetbShowMouseCursor _returnvalue false)
      (Variables|/Script/Engine.PlayerController|SetbEnableMouseOverEvents _returnvalue false)
      (UserInterface|Animation|PlayAnimation _decisionwidget_2 _blendin 0.0 1 "Forward" 1.0)
      (Utilities|FlowControl|Delay (Class|WidgetAnimation|GetEndTime _blendin))
      (Widget|SetVisibility (Variables|/Game/DialogueSystem/Widgets/DecisionDialogue.DecisionDialogue_C|GetTimeLimitBorder _decisionwidget) "Hidden")
      (Widget|SetVisibility _decisionwidget "Hidden")
      (Variables|Default|SetDecisionFinished false)
      (Variables|Default|SetIsCurrentDecision false)
      (Default|OnDecisionMade (Variables|Default|GetCharacter) (Variables|Default|GetCurrentDecisionIndex) (+ (Variables|Default|GetChosenOption) 1))
      (goto _label Reset))))

(event Custom|OnContinueDialogue
  (bind _dialoguewidget (Variables|Default|GetDialogueWidget))
  (bind _blendin (Variables|/Game/DialogueSystem/Widgets/DefaultDialogue.DefaultDialogue_C|GetBlendIn _dialoguewidget))
  ;[1 1 1] On Continue Dialogue
  (Variables|Default|SetWaitingForInput false)
  (UserInterface|Animation|PlayAnimation _dialoguewidget _blendin 0.0 1 "Forward" 1.0)
  (Utilities|FlowControl|Delay (Class|WidgetAnimation|GetEndTime _blendin))
  (Widget|SetVisibility (Variables|Default|GetDialogueWidget) "Hidden")
  (Variables|Default|SetDialogueFinished false)
  (Variables|Default|SetIsCurrentDecision false)
  (Default|OnDialogueFinish (Variables|Default|GetCharacter) (Variables|Default|GetCurrentDialogueIndex)))

(event Custom|OnDecisionSpoken)

(event Custom|AddDecision
  (params (Decision :type S%20Decision%20Information%20Structure) (Index :type Integer))
  (bind _dialogue (Utilities|Struct|BreakS_DecisionInformation Decision))
  (bind (_audiofile _spokentext _sendername _canbeskipped _skiptime) (Utilities|Struct|BreakS_DialogueInformation _dialogue))
  ;[1 1 1] Add Decision Dialogue
  (if (not (Variables|Default|GetIsCurrentDecision))
    (Variables|Default|SetIsCurrentDecision true)
    (Variables|Default|SetCurrentDecisionIndex Index)
    (Utilities|IsValid _audiofile
      (:Is%20Valid
        (bind _returnvalue (Audio|SpawnSound2D _audiofile))
        (Variables|Default|SetCurrentSound _returnvalue)
        (Default|UpdateDialogue (Variables|Default|GetDecisionWidget) Decision)
        (Utilities|FlowControl|Sequence
          (:then_0
            (if _canbeskipped
              (Utilities|FlowControl|Delay _skiptime)
              (Variables|Default|SetWaitingForInput true)
              (Widget|SetVisibility (Variables|/Game/DialogueSystem/Widgets/DecisionDialogue.DecisionDialogue_C|GetSpaceText (Variables|Default|GetDecisionWidget)) "Visible")))
          (:then_1
            (Utilities|FlowControl|Delay (select (Utilities|IsValid _audiofile) (Variables|/Script/Engine.SoundBase|GetDuration _audiofile) 3.0))
            (CallFunction|OnDecisionSpoken)))))))

(event EventBeginPlay
  (bind _hud (Variables|Default|GetHUD))
  ;[1 1 1] Initalize Dialogue Widgets
  (Variables|Default|SetDialogueWidget (Variables|/Game/Widgets/HUD.HUD_C|GetDialogueWidget _hud))
  (Variables|Default|SetDecisionWidget (Variables|/Game/Widgets/HUD.HUD_C|GetDecisionWidget _hud))
  (Variables|/Game/DialogueSystem/Widgets/DecisionDialogue.DecisionDialogue_C|SetDialogueManager (Variables|/Game/Widgets/HUD.HUD_C|GetDecisionWidget _hud) self))

(fn ConstructionScript)