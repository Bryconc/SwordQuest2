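; Base quest actor that tracks one quest's current and completed sub-goals, description and progress state.
; Completing a goal unlocks its following goals, appends description text and syncs the quest widget, sub-goal widgets and journal, with an empty OnGoalCompleted event as a hook.
; AddGoalForIndex recursively auto-completes goals whose target is already among the player's obtained objects.
; Parallel arrays hold goal indices, goal data and hunted counts.
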(event Custom|OnGoalCompleted
  (params (GoalIndex :type Integer)))

(fn ConstructionScript)

(fn UpdateSubGoals
  (Utilities|Array|Clear (Variables|QuestSystemVariables|GetCurrentGoals))
  (for _array_element (Variables|QuestSystemVariables|GetCurrentGoalIndices)
    (Utilities|Array|Add (Variables|QuestSystemVariables|GetCurrentGoals) (Utilities|Array|Get(acopy) (.SubGoals (Utilities|Struct|BreakS_QuestInformation (Variables|QuestInformation|GetQuestInfo))) _array_element)))
  (return))

(fn SetupStartingGoals
  (Utilities|Array|Clear (Variables|QuestSystemVariables|GetCurrentGoalIndices))
  ;[1 1 1] Setup Current Description of Quest
  (Variables|QuestSystemVariables|SetCurrentDescription (.Description (Utilities|Struct|BreakS_QuestInformation (Variables|QuestInformation|GetQuestInfo))))
  (for _array_element (Variables|QuestInformation|GetStartingSubGoalIndices)
    (CallFunction|AddGoalforIndex _array_element)
    (Utilities|Array|Resize (Variables|QuestSystemVariables|GetCurrentHuntedAmounts) (Utilities|Array|Length (Variables|QuestSystemVariables|GetCurrentGoalIndices)))
    (CallFunction|UpdateSubGoals)
    (return)))

(fn GotoNextSubGoal
  (bind _currentgoalindices (Variables|QuestSystemVariables|GetCurrentGoalIndices))
  (bind _currentgoalindices_2 (Variables|QuestSystemVariables|GetCurrentGoalIndices))
  (bind _maxvalue (Math|Integer|MaxOfIntArray _currentgoalindices))
  (bind _returnvalue (+ _maxvalue 1))
  (if (<= _returnvalue (Utilities|Array|LastIndex (.SubGoals (Utilities|Struct|BreakS_QuestInformation (Variables|QuestInformation|GetQuestInfo)))))
    (bind _output_get (LocalVariables|SetNextIndex _returnvalue))
    (Utilities|Array|Clear _currentgoalindices_2)
    (Utilities|Array|Add _currentgoalindices_2 _output_get)
    (CallFunction|UpdateSubGoals)
    (return true)
    (else
      (return false))))

(fn CompleteSubGoal
  (params (SubGoalIndex :type Integer))
  (bind _questwidget (Variables|QuestSystemVariables|GetQuestWidget))
  (bind _questwidget_2 (Variables|QuestSystemVariables|GetQuestWidget))
  (bind _subgoalwidgets (Variables|/Game/QuestSystem/Widgets/QuestWidget.QuestWidget_C|GetSubGoalWidgets _questwidget))
  (bind _output_get (LocalVariables|SetlocalGoalIndex SubGoalIndex))
  (if (Utilities|Array|ContainsItem (Variables|QuestSystemVariables|GetCurrentGoalIndices) _output_get)
    ;[1 1 1] Add Completed Sub Goal
    (bind _output_get_2 (LocalVariables|SetlocalCompletedGoal (Utilities|Array|Get(acopy) (.SubGoals (Utilities|Struct|BreakS_QuestInformation (Variables|QuestInformation|GetQuestInfo))) (LocalVariables|GetlocalGoalIndex))))
    (Utilities|Array|Add (Variables|QuestSystemVariables|GetCompletedSubGoals) (Utilities|Struct|MakeS_CompletedGoal (LocalVariables|GetlocalGoalIndex) (LocalVariables|GetlocalCompletedGoal) true))
    ;[1 1 1] Update Quest Description
    (if (.UpdateQuestDescription (Utilities|Struct|BreakS_GoalInformation (LocalVariables|GetlocalCompletedGoal)))
      (Variables|QuestSystemVariables|SetCurrentDescription (Utilities|Text|FormatText "{Current}{Next}" (Variables|QuestSystemVariables|GetCurrentDescription) (.UpdatedDescription (Utilities|Struct|BreakS_GoalInformation (LocalVariables|GetlocalCompletedGoal)))))
      (if (CallFunction|IsSelectedinJournal)
        (Default|UpdateDescription (Variables|/Game/Widgets/HUD.HUD_C|GetJournal (Variables|/Game/QuestSystem/Blueprints/Actors/BP_QuestManager.BP_QuestManager_C|GetHUD (Variables|QuestSystemVariables|GetQuestManager))))))
    (Utilities|Array|RemoveItem (Variables|QuestSystemVariables|GetCurrentGoals) _output_get_2)
    (LocalVariables|SetlocalWidgetIndex (Utilities|Array|FindItem (Variables|QuestSystemVariables|GetCurrentGoalIndices) (LocalVariables|GetlocalGoalIndex)))
    (Utilities|Array|RemoveIndex (Variables|QuestSystemVariables|GetCurrentHuntedAmounts) (Utilities|Array|FindItem (Variables|QuestSystemVariables|GetCurrentGoalIndices) (LocalVariables|GetlocalGoalIndex)))
    ;[1 1 1] Remove Completed Goal from Current Goals
    (Utilities|Array|RemoveItem (Variables|QuestSystemVariables|GetCurrentGoalIndices) (LocalVariables|GetlocalGoalIndex))
    (Widget|RemovefromParent (Utilities|Array|Get(acopy) _subgoalwidgets (LocalVariables|GetlocalWidgetIndex)))
    (Utilities|Array|RemoveIndex _subgoalwidgets (LocalVariables|GetlocalWidgetIndex))
    (CallFunction|OnGoalCompleted (LocalVariables|GetlocalGoalIndex))
    (for _array_element (.FollowingSubGoalIndices (Utilities|Struct|BreakS_GoalInformation (LocalVariables|GetlocalCompletedGoal)))
      (CallFunction|AddGoalforIndex _array_element))
    ;[1 1 1] Update Sub Goals in Quest Journal
    (if (CallFunction|IsSelectedinJournal)
      (Default|GenerateSubGoals (Variables|/Game/Widgets/HUD.HUD_C|GetJournal (Variables|/Game/QuestSystem/Blueprints/Actors/BP_QuestManager.BP_QuestManager_C|GetHUD (Variables|QuestSystemVariables|GetQuestManager)))))
    ;[1 1 1] Select New Sub Goal
    (if (and (== (LocalVariables|GetlocalGoalIndex) (Variables|QuestSystemVariables|GetSelectedSubGoalIndex)) (== (Variables|/Game/QuestSystem/Blueprints/Actors/BP_QuestManager.BP_QuestManager_C|GetCurrentQuest (Variables|QuestSystemVariables|GetQuestManager)) self))
      (Default|SelectSubGoal _questwidget_2 (Utilities|Array|Get(acopy) (Variables|/Game/QuestSystem/Widgets/QuestWidget.QuestWidget_C|GetSubGoalWidgets _questwidget_2))))
    (return true)
    (else
      (return false))))

(fn IsSelectedinJournal
  (bind _questmanager (Variables|QuestSystemVariables|GetQuestManager))
  (bind _hud (Variables|/Game/QuestSystem/Blueprints/Actors/BP_QuestManager.BP_QuestManager_C|GetHUD _questmanager))
  (bind _journal (Variables|/Game/Widgets/HUD.HUD_C|GetJournal _hud))
  (bind _selectedquest (Variables|/Game/QuestSystem/Widgets/QuestJournal.QuestJournal_C|GetSelectedQuest _journal))
  (return (and (== _selectedquest self) (Utilities|IsValid _selectedquest))))

(fn GoalatIndex
  (params (Index :type Integer))
  (return (Utilities|Array|Get(acopy) (.SubGoals (Utilities|Struct|BreakS_QuestInformation (Variables|QuestInformation|GetQuestInfo))) Index)))

(fn IsGoalAlreadyFound
  (params (GoalIndex :type Integer))
  (bind _goal (CallFunction|GoalatIndex GoalIndex))
  (bind (_type _iscustomgoal _goaltext _additionalname _amounttohunt _goalclass) (Utilities|Struct|BreakS_GoalInformation _goal))
  (if (Utilities|Enum|Equal(Enum) _type "NewEnumerator2")
    (bind _array_element (Utilities|Array|ForEachLoopwithBreak (Variables|/Game/Blueprints/FirstPerson/BP_FirstPersonCharacter.BP_FirstPersonCharacter_C|GetObtainedObjects (Variables|/Game/QuestSystem/Blueprints/Actors/BP_QuestManager.BP_QuestManager_C|GetFirstPersonCharacter (Variables|QuestSystemVariables|GetQuestManager))))
      (:LoopBody
        (if (== _array_element _goalclass)
          (return true)))
      (:Completed
        (return false)))
    (else
      (return false))))

(fn AddGoalforIndex
  (params (Index :type Integer))
  (bind _questwidget (Variables|QuestSystemVariables|GetQuestWidget))
  (bind _output_get (LocalVariables|SetLocalIndex Index))
  (LocalVariables|SetLocalGoal (CallFunction|GoalatIndex (LocalVariables|GetLocalIndex)))
  (if (CallFunction|IsGoalAlreadyFound _output_get)
    (Utilities|Array|Add (Variables|QuestSystemVariables|GetCompletedSubGoals) (Utilities|Struct|MakeS_CompletedGoal (LocalVariables|GetLocalIndex) (LocalVariables|GetLocalGoal) true))
    (CallFunction|OnGoalCompleted (LocalVariables|GetLocalIndex))
    (if (.UpdateQuestDescription (Utilities|Struct|BreakS_GoalInformation (LocalVariables|GetLocalGoal)))
      (Variables|QuestSystemVariables|SetCurrentDescription (Utilities|Text|FormatText "{Current}{Next}" (Variables|QuestSystemVariables|GetCurrentDescription) (.UpdatedDescription (Utilities|Struct|BreakS_GoalInformation (LocalVariables|GetLocalGoal)))))
      (if (CallFunction|IsSelectedinJournal)
        (Default|UpdateDescription (Variables|/Game/Widgets/HUD.HUD_C|GetJournal (Variables|/Game/QuestSystem/Blueprints/Actors/BP_QuestManager.BP_QuestManager_C|GetHUD (Variables|QuestSystemVariables|GetQuestManager))))))
    (for _array_element (.FollowingSubGoalIndices (Utilities|Struct|BreakS_GoalInformation (LocalVariables|GetLocalGoal)))
      (CallFunction|AddGoalforIndex _array_element))
    (return)
    (else
      (bind _returnvalue (Utilities|Array|Add (Variables|QuestSystemVariables|GetCurrentGoalIndices) (LocalVariables|GetLocalIndex)))
      (if (> _returnvalue (Utilities|Array|LastIndex (Variables|QuestSystemVariables|GetCurrentHuntedAmounts)))
        (Utilities|Array|Add (Variables|QuestSystemVariables|GetCurrentHuntedAmounts) 0))
      ;[1 1 1] Create Sub Goal Widget
      (Utilities|Array|Add (Variables|QuestSystemVariables|GetCurrentGoals) (LocalVariables|GetLocalGoal))
      (bind _returnvalue_2 (UserInterface|CreateWidget "/Game/QuestSystem/Widgets/SubGoalWidget.SubGoalWidget_C" 0 (LocalVariables|GetLocalGoal) self (Variables|QuestSystemVariables|GetQuestWidget)))
      (Utilities|Array|Add (Variables|/Game/QuestSystem/Widgets/QuestWidget.QuestWidget_C|GetSubGoalWidgets _questwidget) _returnvalue_2)
      (Widget|Panel|AddChild (Variables|/Game/QuestSystem/Widgets/QuestWidget.QuestWidget_C|GetSubGoalBox _questwidget) _returnvalue_2)
      (return))))

(fn UpdateProgressState
  (params (NewState :type Integer))
  (Variables|QuestInformation|SetCurrentProgressState NewState)
  (return))