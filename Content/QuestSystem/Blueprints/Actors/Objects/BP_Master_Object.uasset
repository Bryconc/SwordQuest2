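; BP_Master_Object is a base interactable pickup for the quest system.
; On begin play it fills its interaction widget with the object name and prompt text, and player-radius events show or hide that widget.
; Interacting adds the object's class to the character's obtained objects, notifies that character's quest manager that it was found, then destroys the actor.
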(event EventOnEnterPlayerRadius
  (params (Character :type BP%20First%20Person%20Character%20Object%20Reference))
  ;[1 1 1] Set Widget Visible on Player Near
  (Rendering|SetVisibility (Variables|Default|GetInteract%20Widget) true false))

(event EventOnLeavePlayerRadius
  (params (Character :type BP%20First%20Person%20Character%20Object%20Reference))
  ;[1 1 1] Set Widget Visible on Player Near
  (Rendering|SetVisibility (Variables|Default|GetInteract%20Widget) false false))

(event EventOnInteractwith
  (params (Character :type BP%20First%20Person%20Character%20Object%20Reference))
  (bind _self self)
  (bind _returnvalue (Utilities|GetClass _self))
  (Utilities|Array|Add (Variables|/Game/Blueprints/FirstPerson/BP_FirstPersonCharacter.BP_FirstPersonCharacter_C|GetObtainedObjects Character) _returnvalue)
  (Default|OnObjectFound (Variables|/Game/Blueprints/FirstPerson/BP_FirstPersonCharacter.BP_FirstPersonCharacter_C|GetQuestManagerReference Character) _returnvalue)
  (Actor|DestroyActor))

(event EventBeginPlay
  (bind _asinteraction_widget (Utilities|Casting|CastToInteractionWidget (UserInterface|GetUserWidgetObject (Variables|Default|GetInteract%20Widget))))
  ;[1 1 1] Set Object Name in Widget
  (Rendering|Components|TextRender|SetText (Variables|/Game/QuestSystem/Widgets/InteractionWidget.InteractionWidget_C|GetName _asinteraction_widget) (Variables|Default|GetObjectName))
  ;[1 1 1] Set Interact Text
  (Rendering|Components|TextRender|SetText (Variables|/Game/QuestSystem/Widgets/InteractionWidget.InteractionWidget_C|GetInteractionText _asinteraction_widget) (Variables|Default|GetInteractText)))

(fn ConstructionScript)