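; BP_QuestManager is the quest manager actor that adds, selects and progresses the player's quests.
; AddNewQuest spawns one actor per unique quest class, registers it with the HUD list and journal, and selects it if first or requested.
; Object-found and enemy-killed events scan active quests for matching goal classes, completing sub-goals or incrementing hunt counts and refreshing their widgets.
; Switching sub-quests destroys any existing goal actor, otherwise caches the selected sub-goal.
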(event Custom|OnSwitchSubQuest
  (bind _currentquest (Variables|Default|GetCurrentQuest))
  (Utilities|IsValid (Variables|Default|GetCurrentGoalActor)
    (:Is%20Valid
      (Actor|DestroyActor (Variables|Default|GetCurrentGoalActor)))
    (:Is%20Not%20Valid
      (bind _output_get (Variables|Default|SetCurrentSubGoal (Utilities|Array|Get(acopy) (.SubGoals (Utilities|Struct|BreakS_QuestInformation (Variables|/Game/QuestSystem/Blueprints/Actors/QuestActors/BP_MasterQuest.BP_MasterQuest_C|GetQuestInfo _currentquest))) (Variables|/Game/QuestSystem/Blueprints/Actors/QuestActors/BP_MasterQuest.BP_MasterQuest_C|GetSelectedSubGoalIndex _currentquest))))
      (if (not true)
        (Variables|Default|SetCurrentGoalActor 0)))))

(event Custom|OnEnemyKilled
  (params (Class :type Actor%20Class%20Reference))
  (bind _output_get (Variables|Default|SetKilledEnemy Class))
  (for _array_element (Variables|Default|GetCurrentQuestActors)
    (for (_array_element_2 _array_index) (Variables|/Game/QuestSystem/Blueprints/Actors/QuestActors/BP_MasterQuest.BP_MasterQuest_C|GetCurrentGoals _array_element)
      (if (and (Utilities|Enum|Equal(Enum) (.Type (Utilities|Struct|BreakS_GoalInformation _array_element_2)) "NewEnumerator1") (== (.GoalClass (Utilities|Struct|BreakS_GoalInformation _array_element_2)) _output_get))
        (if (>= (+ (Utilities|Array|Get(acopy) (Variables|/Game/QuestSystem/Blueprints/Actors/QuestActors/BP_MasterQuest.BP_MasterQuest_C|GetCurrentHuntedAmounts _array_element) _array_index) 1) (.AmountToHunt (Utilities|Struct|BreakS_GoalInformation _array_element_2)))
          (Default|CompleteSubGoal _array_element (Utilities|Array|Get(acopy) (Variables|/Game/QuestSystem/Blueprints/Actors/QuestActors/BP_MasterQuest.BP_MasterQuest_C|GetCurrentGoalIndices _array_element) _array_index))
          (else
            (Utilities|Array|SetArrayElem (Variables|/Game/QuestSystem/Blueprints/Actors/QuestActors/BP_MasterQuest.BP_MasterQuest_C|GetCurrentHuntedAmounts _array_element) _array_index (+ (Utilities|Array|Get(acopy) (Variables|/Game/QuestSystem/Blueprints/Actors/QuestActors/BP_MasterQuest.BP_MasterQuest_C|GetCurrentHuntedAmounts _array_element) _array_index) 1))
            (Default|Update (Utilities|Array|Get(acopy) (Variables|/Game/QuestSystem/Widgets/QuestWidget.QuestWidget_C|GetSubGoalWidgets (Variables|/Game/QuestSystem/Blueprints/Actors/QuestActors/BP_MasterQuest.BP_MasterQuest_C|GetQuestWidget _array_element)) _array_index))
            (if true
              (Default|GenerateSubGoals (Variables|/Game/Widgets/HUD.HUD_C|GetJournal (Variables|Default|GetHUD))))))))))

(event Custom|OnObjectFound
  (params (FoundObject :type BP%20Master%20Object%20Class%20Reference))
  (Variables|Default|SetFoundObject FoundObject)
  (for _array_element (Variables|Default|GetCurrentQuestActors)
    (for (_array_element_2 _array_index) (Variables|/Game/QuestSystem/Blueprints/Actors/QuestActors/BP_MasterQuest.BP_MasterQuest_C|GetCurrentGoals _array_element)
      (if (and (Utilities|Enum|Equal(Enum) (.Type (Utilities|Struct|BreakS_GoalInformation _array_element_2)) "NewEnumerator2") (== (.GoalClass (Utilities|Struct|BreakS_GoalInformation _array_element_2)) (Variables|Default|GetFoundObject)))
        (Default|CompleteSubGoal _array_element (Utilities|Array|Get(acopy) (Variables|/Game/QuestSystem/Blueprints/Actors/QuestActors/BP_MasterQuest.BP_MasterQuest_C|GetCurrentGoalIndices _array_element) _array_index))))))

(fn ConstructionScript)

(fn SelectNewQuest
  (params (Quest :type BP%20Master%20Quest%20Object%20Reference) (SubGoal :type Sub%20Goal%20Widget%20Object%20Reference))
  (Utilities|IsValid (Variables|Default|GetCurrentQuest)
    (:Is%20Valid
      (Widget|SetIsEnabled (Variables|/Game/QuestSystem/Widgets/QuestWidget.QuestWidget_C|GetQuestName (Variables|/Game/QuestSystem/Blueprints/Actors/QuestActors/BP_MasterQuest.BP_MasterQuest_C|GetQuestWidget (Variables|Default|GetCurrentQuest))) false)
      (Default|SelectSubGoal (Variables|/Game/QuestSystem/Blueprints/Actors/QuestActors/BP_MasterQuest.BP_MasterQuest_C|GetQuestWidget (Variables|Default|GetCurrentQuest))))
    (:Is%20Not%20Valid
      _))
  (bind _output_get (Variables|Default|SetCurrentQuest Quest))
  (Default|OnQuestSelected (Variables|/Game/QuestSystem/Blueprints/Actors/QuestActors/BP_MasterQuest.BP_MasterQuest_C|GetQuestWidget _output_get) SubGoal)
  (return))

(fn AddNewQuest
  (params (QuestClass :type BP%20Master%20Quest%20Class%20Reference) (ShouldDirectlyStart :type Boolean))
  (bind _hud (Variables|Default|GetHUD))
  (LocalVariables|SetLocalShouldStart ShouldDirectlyStart)
  (bind _output_get (LocalVariables|SetLocalClass QuestClass))
  (if (and (Utilities|IsValidClass QuestClass) (not (Utilities|Array|ContainsItem (Variables|Default|GetAllQuestClasses) QuestClass)))
    (Utilities|Array|Add (Variables|Default|GetAllQuestClasses) _output_get)
    (bind _returnvalue (Game|SpawnActorfromClass _output_get (Math|Transform|MakeTransform "0, 0, 0" "0, 0, 0" "1,1.000000,1") "AlwaysSpawn" 0 self 0))
    (bind _output_get_2 (LocalVariables|SetLocalQuestActor _returnvalue))
    (Utilities|Array|Add (Variables|Default|GetCurrentQuestActors) _output_get_2)
    (bind _questwidget (Default|AddQuesttoList (Variables|/Game/Blueprints/FirstPerson/BP_FirstPersonCharacter.BP_FirstPersonCharacter_C|GetHUDReference (Variables|Default|GetFirstPersonCharacter)) (LocalVariables|GetLocalQuestActor)))
    (bind _output_get_3 (Variables|/Game/QuestSystem/Blueprints/Actors/QuestActors/BP_MasterQuest.BP_MasterQuest_C|SetQuestWidget (LocalVariables|GetLocalQuestActor) _questwidget))
    (Default|SetupStartingGoals (LocalVariables|GetLocalQuestActor))
    (Default|UpdateQuest _output_get_3)
    ;[1 1 1] Add New Quest to Quest Journal
    (Default|AddEntry (Variables|/Game/Widgets/HUD.HUD_C|GetJournal (Variables|Default|GetHUD)) (LocalVariables|GetLocalQuestActor))
    ;[1 1 1] Select the Added Quest if Only Quest or Should Start
    (if (or (LocalVariables|GetLocalShouldStart) (<= (Utilities|Array|Length (Variables|Default|GetCurrentQuestActors)) 1))
      (CallFunction|SelectNewQuest (LocalVariables|GetLocalQuestActor) (Utilities|Array|Get(acopy) (Variables|/Game/QuestSystem/Widgets/QuestWidget.QuestWidget_C|GetSubGoalWidgets (Variables|/Game/QuestSystem/Blueprints/Actors/QuestActors/BP_MasterQuest.BP_MasterQuest_C|GetQuestWidget (LocalVariables|GetLocalQuestActor))))))
    ;[1 1 1] Slide out Quest Journal if Not Already Visible
    (if (Variables|/Game/Widgets/HUD.HUD_C|GetDidSlideOut (Variables|Default|GetHUD))
      (UserInterface|Animation|PlayAnimation _hud (Variables|/Game/Widgets/HUD.HUD_C|GetSlideOut _hud) 0.0 1 "Reverse" 1.0)
      (Variables|/Game/Widgets/HUD.HUD_C|SetDidSlideOut _hud false))
    (return true)
    (else
      (return false))))